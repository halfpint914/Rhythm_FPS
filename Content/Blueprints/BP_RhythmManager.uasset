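; BP_RhythmManager runs the beat clock for a shooter and judges whether player actions land on beat.
; After a short startup delay, it adds a crosshair widget and starts a looping quarter-beat timer derived from BPM.
; The four-step cycle feeds the crosshair and records beat time on its last step.
; Shot, reload and dash events compare their timing to the nearest beat within a tolerance window, giving debug text and sound feedback.
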(event `Register Reload`
  ;[0.6521 0.6562 0.06836 0.5] BPM Audio
  (bind _wasonbeat (`self.EvaluateShot` :!label _label))
  (bind _output_get (set `self.Was on Beat?` _wasonbeat))
  (if _output_get
    (if true
      (`KismetSystemLibrary.PrintString` "ON BEAT!")
      (`GameplayStatics.PlaySound2D` "/Game/Audio/Dark_Click_A.Dark_Click_A" 1.0 1.0 0.0 null null))
    (else
      (`KismetSystemLibrary.PrintString` "Not QUITE my tempo.")
      (`GameplayStatics.PlaySound2D` "/Game/Audio/Dark_Subtle_Hover_B.Dark_Subtle_Hover_B" 1.0 1.0 0.0 null null))))

(event `RegisterShot`
  ;[0.6521 0.6562 0.06836 0.5] BPM Audio
  (goto _label))

(event `RegisterDash`
  ;[0.6521 0.6562 0.06836 0.5] BPM Audio
  (goto _label))

(event `OnBeat`
  ;[0.6521 0.6562 0.06836 0.5] BPM Audio
  (set `self.LastBeatTime` (`KismetSystemLibrary.GetGameTimeInSeconds`))
  (`KismetSystemLibrary.PrintString` "BEAT" true true (struct :`R` 0.427106 :`G` 0.106273 :`B` 1.0 :`A` 1.0))
  (`GameplayStatics.PlaySound2D` "/Game/Audio/Phat_Subtle_Hover_B.Phat_Subtle_Hover_B" 1.0 1.0 0.0 null null))

(event `BPM Set`
  (bind _output_get (set `self.BeatInterval` (/ 60.0 (`self.BPM`))))
  (set `self.SubdivisionInterval` (/ _output_get 4.0))
  (set `self.BeatStartTime` (`KismetSystemLibrary.GetGameTimeInSeconds`))
  ;[0.15 1 0.15 0.5] BPM Rhythm
  (`KismetSystemLibrary.Delay` 0.2 :!label _label_2)
  (bind _output_get_2 (set `self.BeatInterval` (/ 60.0 (`self.BPM`))))
  (set `self.SubdivisionInterval` (/ _output_get_2 4.0))
  (set `self.BeatStartTime` (`KismetSystemLibrary.GetGameTimeInSeconds`))
  ;[0.2006 0.02417 0.5156] Add Reticle HUD to Viewport
  (bind _returnvalue (`|CreateWidget` "/Game/Blueprints/WBP_RhythmCrosshair.WBP_RhythmCrosshair_C" (`GameplayStatics.GetPlayerController` 0)))
  (bind _output_get_3 (set `self.RhythmCrosshair` _returnvalue))
  (`UserWidget.AddToViewport` _output_get_3 0)
  (`self.ProcessRhythmStep`)
  (`KismetSystemLibrary.K2_SetTimerDelegate` (`|CreateDelegate` :!event `AdvanceRhythmStep`) (`self.SubdivisionInterval`) true))

(event `self.ReceiveBeginPlay`
  (bind _asbp_shooter_character (cast `/Game/Variant_Shooter/Blueprints/BP_ShooterCharacter` (`GameplayStatics.GetPlayerCharacter` 0)))
  (set `self.Main Character REF` _asbp_shooter_character)
  (goto _label_2))

(event `ProcessRhythmStep`
  (bind _rhythmcrosshair (`self.RhythmCrosshair`))
  (bind _currentrhythmstep (`self.CurrentRhythmStep`))
  ;[0 0.1142 0.5625 0.5] Current Rhythm Process
  (`/Engine/EditorBlueprintResources/StandardMacros.IsValid` _rhythmcrosshair
    (:`Is Valid`
      (`/Game/Blueprints/WBP_RhythmCrosshair.SetRhythmStep` _rhythmcrosshair _currentrhythmstep)
      (if (== _currentrhythmstep 3)
        (`self.OnBeat`)))))

(event `AdvanceRhythmStep`
  ;[0.5521 0.03048 0.3849 0.5] AdvanceRhythmStep
  (set `self.CurrentRhythmStep` (mod (+ (`self.CurrentRhythmStep`) 1) 4))
  (`self.ProcessRhythmStep`))

(fn `EvaluateShot`
  (returns (WasOnBeat :type Boolean))
  (bind _returnvalue (- (`KismetSystemLibrary.GetGameTimeInSeconds`) (`self.LastBeatTime`)))
  (return (<= (`KismetMathLibrary.FMin` _returnvalue (- (`self.BeatInterval`) (mod _returnvalue (`self.BeatInterval`)))) (`self.OnBeatWindow`))))

(fn `UserConstructionScript`)