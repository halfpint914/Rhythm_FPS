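; BP_SongPlayer starts the selected song for a level in a rhythm shooter and ends the level when the track finishes.
; On BeginPlay it uses the game instance's song index to look up DT_Song, pass BPM to BP_RhythmManager, give the character the song name and play the audio.
; When audio finishes, it shows WBP_LevelComplete with the player's score, switches to UI-only input and pauses the game.
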(event `self.ReceiveBeginPlay`
  (bind _asbp_shooter_character (cast `/Game/Variant_Shooter/Blueprints/BP_ShooterCharacter` (`GameplayStatics.GetPlayerCharacter` 0)))
  (set `self.Character REF` _asbp_shooter_character)
  (bind _returnvalue (`GameplayStatics.GetActorOfClass` "/Game/Blueprints/BP_RhythmManager.BP_RhythmManager_C"))
  (bind _asbp_rhythm_manager (cast `/Game/Blueprints/BP_RhythmManager` _returnvalue))
  (set `self.Rhythm Manager REF` _asbp_rhythm_manager)
  (bind _asgi_rhythm_shooter (cast `/Game/Blueprints/GI_RhythmShooter` (`GameplayStatics.GetGameInstance`)))
  (set `self.Rhythm Shooter GI` _asgi_rhythm_shooter)
  (`self.Play Song`))

(event `Play Song`
  (bind _rhythm_manager_ref (`self.Rhythm Manager REF`))
  (bind _output_get (set `self.Row Name` (`.Value` (`BlueprintMapLibrary.Map_GetKeyValueByIndex` (`self.Track Number`) (`/Game/Blueprints/GI_RhythmShooter.Selected Song Index` (`self.Rhythm Shooter GI`))))))
  (`KismetSystemLibrary.Delay` 0.1)
  (bind _returnvalue (`|GetDataTableRow` "/Game/Blueprints/Songs/DT_Song.DT_Song" _output_get)
    (:`then`
      (set `/Game/Blueprints/BP_RhythmManager.BPM` (`.BPM_5_27A600B444C91A778435FF9199474B30` (break `/Game/Blueprints/Songs/S_Song` _returnvalue)) _rhythm_manager_ref)
      (`/Game/Blueprints/BP_RhythmManager.BPM Set` _rhythm_manager_ref)
      (`/Game/Variant_Shooter/Blueprints/BP_ShooterCharacter.Set Song Name` (`self.Character REF`) (`.NameofSong_11_A1DBF56149F6CD80A28EA293650D57D9` (break `/Game/Blueprints/Songs/S_Song` _returnvalue)))
      (bind _returnvalue_2 (`GameplayStatics.SpawnSound2D` (break `/Game/Blueprints/Songs/S_Song` _returnvalue) 0.5 1.0 0.0 null))
      (bind _output_get_2 (set `self.Current Level Song` _returnvalue_2))
      (add `AudioComponent.OnAudioFinished` _output_get_2 (delegate `OnAudioFinished_Event`)))))

(event `OnAudioFinished_Event`
  (bind _returnvalue (`GameplayStatics.GetPlayerController` 0))
  (bind _player_score (`/Game/Variant_Shooter/Blueprints/BP_ShooterCharacter.Player Score` (`self.Character REF`)))
  (bind _returnvalue_2 (`|CreateWidget` "/Game/Widgets/WBP_LevelComplete.WBP_LevelComplete_C" _returnvalue))
  (bind _output_get (set `self.Level Complete Widget` _returnvalue_2))
  (`UserWidget.AddToViewport` _output_get 0)
  (`WidgetBlueprintLibrary.SetInputMode_UIOnlyEx` _returnvalue _output_get)
  (if (>= _player_score (stale _output_get_2))
    (bind _output_get_2 (set `self.Current Index` (`.Value` (`BlueprintMapLibrary.Map_GetKeyValueByIndex` (`/Game/Blueprints/GI_RhythmShooter.Song List Score` (`self.Rhythm Shooter GI`)) (`/Game/Blueprints/GI_RhythmShooter.Selected Song Index` (`self.Rhythm Shooter GI`)))))))
  (`TextBlock.SetText` (`/Game/Widgets/WBP_LevelComplete.LevelScore` (`self.Level Complete Widget`)) (`KismetTextLibrary.Conv_IntToText` _player_score))
  (set `PlayerController.bShowMouseCursor` true (`GameplayStatics.GetPlayerController` 0))
  (`GameplayStatics.SetGamePaused` true))

(fn `UserConstructionScript`)