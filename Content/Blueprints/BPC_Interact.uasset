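; Player interaction component for BP_FirstPersonCharacter that handles key pickup, locked doors, path-moving objects and phase objects, and creates the key and player HUDs.
; A left-click camera trace collects keys or opens doors, updating the key HUD and playing sounds.
; A prototype per-Tick trace tracks and highlights the focused move or phase object.
; Left-click moves or phases it, release reverses movement, and right-click freezes it.
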(event `self.ReceiveBeginPlay`
  ;[0 0 0 0.5 28] Camera Connection to Line Trace
  (bind _asbp_first_person_character (cast `/Game/FirstPerson/Blueprints/BP_FirstPersonCharacter` (`self.GetOwner`)))
  (set `self.First Person Camera` (`/Game/FirstPerson/Blueprints/BP_FirstPersonCharacter.FirstPersonCamera` _asbp_first_person_character))
  (bind _returnvalue (`|CreateWidget` "/Game/Blueprints/WBP_KeyHUD.WBP_KeyHUD_C" (`GameplayStatics.GetPlayerController` 0)))
  (set `self.KeyHUD` _returnvalue)
  (`UserWidget.AddToViewport` (`self.KeyHUD`) 0)
  (bind _returnvalue_2 (`|CreateWidget` "/Game/Blueprints/WBP_PlayerHUD.WBP_PlayerHUD_C" (`GameplayStatics.GetPlayerController` 0)))
  (set `self.PlayerHUD` _returnvalue_2)
  (`UserWidget.AddToViewport` (`self.PlayerHUD`) 0))

(event `PlayCinematicMessage`
  (params (Message :type Text))
  (bind _playerhud (`self.PlayerHUD`))
  ;[0.401 0.224 0.02298 0.5] Play Cinematic
  (`/Engine/EditorBlueprintResources/StandardMacros.IsValid` _playerhud
    (:`Is Valid`
      (`/Game/Blueprints/WBP_PlayerHUD.ShowCinematicMessage` _playerhud Message))))

(event `Try to Interact`
  (bind _first_person_camera (`self.First Person Camera`))
  (bind _returnvalue (`SceneComponent.K2_GetComponentLocation` _first_person_camera))
  ;[0 0.1138 0.599 0.5 32] Line Trace Functionality
  (bind (_outhit _returnvalue_2) (`KismetSystemLibrary.LineTraceSingle` :`Start` _returnvalue :`End` (+ _returnvalue (* (`SceneComponent.GetForwardVector` _first_person_camera) (`self.LookDistance`))) :`TraceChannel` "TraceTypeQuery1" :`DrawDebugType` "ForDuration"))
  (if _returnvalue_2
    (bind (_bblockinghit _binitialoverlap _time _distance _location _impactpoint _normal _impactnormal _physmat _hitactor) (`GameplayStatics.BreakHitResult` _outhit))
    ;[0.4271 0.3644 0.01112 0.5 28] Key Collect & Destroy
    (bind _asbp_key (cast `/Game/Blueprints/BP_Key` _hitactor)
      (:`then`
        (set `self.HasKey` true)
        (`/Game/Blueprints/WBP_KeyHUD.SetKeyVisible` (`self.KeyHUD`) true)
        (`Actor.K2_DestroyActor` _asbp_key)
        (`KismetSystemLibrary.PrintText` (`|FormatText` "Key ACQUIRED!"))
        (`GameplayStatics.PlaySound2D` "/Game/Audio/Keys_Jingle_A.Keys_Jingle_A" 1.0 1.0 0.0 null null))
      (:`CastFailed`
        ;[0.02638 0.06771 0.02116 0.5] Locked Door Interaction
        (bind _asbp_locked_door (cast `/Game/Blueprints/BP_LockedDoor` _hitactor))
        (if (`self.HasKey`)
          (`GameplayStatics.PlaySound2D` "/Game/Audio/Sharp_Hit.Sharp_Hit" 0.85 1.25 0.5 null null)
          (`Actor.K2_DestroyActor` _asbp_locked_door)
          (set `self.HasKey` false)
          (`/Game/Blueprints/WBP_KeyHUD.SetKeyVisible` (`self.KeyHUD`) false)
          (else
            (`GameplayStatics.PlaySound2D` "/Game/Audio/Metal_Door_Handle_D.Metal_Door_Handle_D" 1.0 1.0 0.0 null null)
            (`KismetSystemLibrary.PrintString` "Door LOCKED!")))))))

(event `Key|LeftMouseButton`
  (params (Key :type "Key Structure"))
  ;[0 0.1138 0.599 0.5 32] Line Trace Functionality
  (:`Pressed`
    (`self.Try to Interact`)))

(event `Key|LeftMouseButton`
  (params (Key :type "Key Structure"))
  (bind _activemoveobject (`self.ActiveMoveObject`))
  ;[0.04158 0.02035 0.1302 0.5] Movable Object Controls
  (:`Pressed`
    (`/Engine/EditorBlueprintResources/StandardMacros.IsValid` (`self.FocusedMoveObject`)
      (:`Is Valid`
        (bind _output_get (set `self.ActiveMoveObject` (`self.FocusedMoveObject`)))
        (`/Game/Blueprints/BP_PathMoveObject.MoveForward` _output_get))
      (:`Is Not Valid`
        (`/Engine/EditorBlueprintResources/StandardMacros.IsValid` (`self.FocusedPhaseObject`)
          (:`Is Valid`
            (set `self.ActiveMoveObject` null)
            (`/Game/Blueprints/BP_PhaseObject.TogglePhase` (`self.FocusedPhaseObject`)))))))
  (:`Released`
    (`/Engine/EditorBlueprintResources/StandardMacros.IsValid` _activemoveobject
      (:`Is Valid`
        (`/Game/Blueprints/BP_PathMoveObject.MoveReverse` _activemoveobject)))))

(event `Key|RightMouseButton`
  (params (Key :type "Key Structure"))
  (bind _activemoveobject (`self.ActiveMoveObject`))
  ;[0.04158 0.02035 0.1302 0.5] Movable Object Controls
  (:`Pressed`
    (`/Engine/EditorBlueprintResources/StandardMacros.IsValid` _activemoveobject
      (:`Is Valid`
        (`/Game/Blueprints/BP_PathMoveObject.FreezeMovement` _activemoveobject)))))

(event `self.ReceiveTick`
  (params (DeltaSeconds :type "Float (single-precision)"))
  (bind _focusedmoveobject (`self.FocusedMoveObject`))
  (bind _first_person_camera (`self.First Person Camera`))
  (bind _focusedmoveobject_2 (`self.FocusedMoveObject`))
  (bind _focusedphaseobject (`self.FocusedPhaseObject`))
  (bind _returnvalue (`SceneComponent.K2_GetComponentLocation` _first_person_camera))
  ;[0.08545 0.5252 0.5469 0.5] Moving Object
  (bind (_outhit _returnvalue_2) (`KismetSystemLibrary.LineTraceSingle` :`Start` _returnvalue :`End` (+ _returnvalue (* (`SceneComponent.GetForwardVector` _first_person_camera) (`self.LookDistanceHighlight`))) :`TraceChannel` "TraceTypeQuery1" :`DrawDebugType` "ForOneFrame"))
  (if _returnvalue_2
    (bind (_bblockinghit _binitialoverlap _time _distance _location _impactpoint _normal _impactnormal _physmat _hitactor) (`GameplayStatics.BreakHitResult` _outhit))
    (set `self.CurrentFocusedActor` _hitactor)
    (bind _asbp_path_move_object (cast `/Game/Blueprints/BP_PathMoveObject` _hitactor) ; NEW OBJECT: Currently Under Crosshair
      (:`then`
        (if (not (== _asbp_path_move_object (`self.FocusedMoveObject`)))
          (`/Engine/EditorBlueprintResources/StandardMacros.IsValid` (`self.FocusedMoveObject`)
            (:`Is Valid`
              (`/Game/Blueprints/BP_PathMoveObject.SetFocused` (`self.FocusedMoveObject`) false))
            (:`Is Not Valid`
              (bind _output_get (set `self.FocusedMoveObject` _asbp_path_move_object))
              (`/Game/Blueprints/BP_PathMoveObject.SetFocused` _output_get true)))))
      (:`CastFailed`
        (`|ExecutionSequence`
          (:`then_0`
            (`/Engine/EditorBlueprintResources/StandardMacros.IsValid` _focusedmoveobject_2
              (:`Is Valid`
                (`/Game/Blueprints/BP_PathMoveObject.SetFocused` _focusedmoveobject_2 false)
                (set `self.FocusedMoveObject` null))))
          (:`then_1`
            ;[0.4722 0.09718 0.7865 0.5] Phase Object
            (bind _asbp_phase_object (cast `/Game/Blueprints/BP_PhaseObject` _hitactor) ; The NEW
              (:`then`
                (if (not (== _asbp_phase_object _focusedphaseobject))
                  (`/Engine/EditorBlueprintResources/StandardMacros.IsValid` _focusedphaseobject
                    (:`Is Valid`
                      (`/Game/Blueprints/BP_PhaseObject.SetFocused` (`self.FocusedPhaseObject`) false)
                      (bind _output_get_2 (set `self.FocusedPhaseObject` _asbp_phase_object))
                      (`/Game/Blueprints/BP_PhaseObject.SetFocused` _output_get_2 true))
                    (:`Is Not Valid`
                      (bind _output_get_3 (set `self.FocusedPhaseObject` _asbp_phase_object))
                      (`/Game/Blueprints/BP_PhaseObject.SetFocused` _output_get_3 true)))))
              (:`CastFailed`
                (`/Engine/EditorBlueprintResources/StandardMacros.IsValid` _focusedphaseobject
                  (:`Is Valid`
                    (`/Game/Blueprints/BP_PhaseObject.SetFocused` _focusedphaseobject false)
                    (set `self.FocusedPhaseObject` null)))))))))
    (else
      (set `self.CurrentFocusedActor` null)
      (`/Engine/EditorBlueprintResources/StandardMacros.IsValid` _focusedmoveobject
        (:`Is Valid`
          (`/Game/Blueprints/BP_PathMoveObject.SetFocused` _focusedmoveobject false)
          (set `self.FocusedMoveObject` null))))))