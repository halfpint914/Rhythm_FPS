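; BP_PathMoveObject is an actor whose mesh slides between its start position and an offset end position, with a highlight when focused.
; BeginPlay creates a dynamic material instance and caches both endpoints in relative space.
; MoveForward, MoveReverse and FreezeMovement drive a timeline that lerps the mesh location, so motion can pause and reverse midway.
; SetFocused plays or reverses a second timeline that fades the material's HighlightStrength parameter.
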(event `self.ReceiveBeginPlay`
  ;[0.04219 0.1207 0.15 0.5] Material Focus
  (bind _returnvalue (`PrimitiveComponent.CreateDynamicMaterialInstance` (`self.MovableMesh`) 0 "/Game/Extras/Materials/M_MovableObject.M_MovableObject" "None"))
  (set `self.MovableMID` _returnvalue)
  (set `self.StartLocation` (`SceneComponent.RelativeLocation` (`self.MovableMesh`)))
  (set `self.EndLocation` (+ (`self.StartLocation`) (`self.MoveOffset`))))

(event `MoveForward`
  ;[0.04219 0.1207 0.15 0.5] Material Focus
  (bind (_direction _movealpha) (`Timeline|TL_Move` :!label _label)
    (:`Update`
      (`SceneComponent.K2_SetRelativeLocation` (`self.MovableMesh`) (`KismetMathLibrary.VLerp` (`self.StartLocation`) (`self.EndLocation`) _movealpha) false false))))

(event `FreezeMovement`
  ;[0.04219 0.1207 0.15 0.5] Material Focus
  (goto _label :!via `Stop`))

(event `MoveReverse`
  ;[0.04219 0.1207 0.15 0.5] Material Focus
  (goto _label :!via `Reverse`))

(event `SetFocused`
  (params (Focused :type Boolean))
  ;[0.3177 0.2796 0.04799 0.5] Material Animated
  (if Focused
    (bind (_direction _highlightalpha) (`Timeline|TL_Highlight` :!label _label_2)
      (:`Update`
        (`MaterialInstanceDynamic.SetScalarParameterValue` (`self.MovableMID`) "HighlightStrength" _highlightalpha)))
    (else
      (goto _label_2 :!via `Reverse`))))

(fn `UserConstructionScript`)